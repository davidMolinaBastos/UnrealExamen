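; SphereBP is a physics-style actor that gets pushed away from the character touching it.
; A Sphere overlap or StaticMeshComponent hit runs shared logic, where the Player flag selects a cast to ThirdPersonCharacterExamen or ThirdPersonCharacter.
; A successful cast applies an impulse to the mesh along the character-to-actor offset, scaled by distance.
; The hit path reuses the overlap event's OtherActor rather than its own.
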(event `self.Sphere.OnComponentBeginOverlap`
  (params (OverlappedComponent :type "PrimitiveComponent Object Reference") (OtherActor :type "Actor Object Reference") (OtherComp :type "PrimitiveComponent Object Reference") (OtherBodyIndex :type Integer) (bFromSweep :type Boolean) (SweepResult :type "HitResult Structure (by ref)"))
  (if (`self.Player`) :!label _label
    (cast `/Game/Examen/ThirdPersonCharacterExamen` OtherActor)
    (else
      (cast `/Game/ThirdPersonBP/Blueprints/ThirdPersonCharacter` OtherActor)))
  (`PrimitiveComponent.AddImpulse` (`self.StaticMeshComponent`) (* (- (`self.K2_GetActorLocation`) (`self.K2_GetActorLocation` OtherActor)) 100.0) "None" false))

(event `self.StaticMeshComponent.OnComponentHit`
  (params (HitComponent :type "PrimitiveComponent Object Reference") (OtherActor :type "Actor Object Reference") (OtherComp :type "PrimitiveComponent Object Reference") (NormalImpulse :type "Vector Structure") (Hit :type "HitResult Structure (by ref)"))
  (goto _label))

(fn `UserConstructionScript`)